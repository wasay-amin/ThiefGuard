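; Game mode for a multiplayer guards-versus-thieves game that assigns roles to joining players and spawns the key, lock and path actors.
; On login, the first two players possess newly spawned Guards and the next three possess faster Thieves.
; BeginPlay places the objective actors at fixed locations and caches the game state.
; A delayed relock event respawns the lock and key and prints a "Door Locked Again!" instruction through the game state.
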(event `self.K2_PostLogin`
  (params (NewPlayer :type "PlayerController Object Reference"))
  (`KismetArrayLibrary.Array_Add` (`self.playerController`) NewPlayer)
  (if (< (`self.noOfGuards`) 2)
    (bind _returnvalue (`|SpawnActorFromClass` "/Game/BluePrint/Character/guard.guard_C" (`KismetMathLibrary.MakeTransform` (0.0 0.0 200.0)) "Undefined" "OverrideRootScale" null null))
    (set `CharacterMovementComponent.MaxWalkSpeed` 400.0 (`Character.CharacterMovement` _returnvalue))
    (`/Engine/EditorBlueprintResources/StandardMacros.IncrementInt` (`self.noOfGuards`)
      (:`  `
        (`Controller.Possess` NewPlayer _returnvalue)
        (if (== (+ (`self.noOfGuards`) (`self.noOfThieves`)) 5) :!label _label
          _)))
    (elif (< (`self.noOfThieves`) 3)
      (bind _returnvalue_2 (`|SpawnActorFromClass` "/Game/BluePrint/Character/thief.thief_C" (`KismetMathLibrary.MakeTransform` (0.0 0.0 200.0)) "Undefined" "OverrideRootScale" null null))
      (set `CharacterMovementComponent.MaxWalkSpeed` 700.0 (`Character.CharacterMovement` _returnvalue_2))
      (`/Engine/EditorBlueprintResources/StandardMacros.IncrementInt` (`self.noOfThieves`)
        (:`  `
          (`Controller.Possess` NewPlayer _returnvalue_2)
          (goto _label))))))

(event `self.ReceiveBeginPlay`
  (`self.spawnedKey`)
  (`self.spawnPath`)
  (`self.spawnLock`)
  (bind _asmy_game_state (cast `/Game/BluePrint/myGameState` (`GameplayStatics.GetGameState`))))

(event `SpawnLockDelay`
  (`KismetSystemLibrary.Delay` 10.0)
  (`self.spawnLock`)
  (`/Game/BluePrint/myGameState.printInstruction` (stale `self.ReceiveBeginPlay` _asmy_game_state) "Door Locked Again!")
  (`self.spawnedKey`))

(fn `spawnedKey`
  (bind _returnvalue (`|SpawnActorFromClass` "/Game/BluePrint/Actor/Key.Key_C" (`KismetMathLibrary.MakeTransform` (2377.655273 45.582729 191.10347) (struct) (0.236 0.236 0.236)) "Undefined" "OverrideRootScale" null null))
  (set `self.key` _returnvalue))

(fn `spawnLock`
  (bind _returnvalue (`|SpawnActorFromClass` "/Game/BluePrint/Actor/lock.lock_C" (`KismetMathLibrary.MakeTransform` (2297.824707 2079.541748 320.921082) (struct) (0.5 0.5 0.5)) "Undefined" "OverrideRootScale" null null))
  (set `self.lock` _returnvalue))

(fn `spawnPath`
  (bind _returnvalue (`|SpawnActorFromClass` "/Game/BluePrint/Actor/path.path_C" (`KismetMathLibrary.MakeTransform` (2389.422852 -2129.446045 200.0) (struct :`Pitch` 50.0)) "Undefined" "OverrideRootScale" null null))
  (set `self.path` _returnvalue))

(fn `UserConstructionScript`)