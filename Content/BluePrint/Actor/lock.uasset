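; Jail lock actor that tells the player-controlled thief whether the jail can be unlocked.
; On Box overlap, it checks the key-collected flag in myGameState and prints either an unlock prompt or a reminder to collect the key.
; With the key, it also sets an in-range flag on the thief; the unlock itself is not handled here, and nothing clears that flag on leaving.
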(event `self.ReceiveBeginPlay`
  ;[1 1 1] Game Mode & Game State
  (bind _asmy_game_mode (cast `/Game/BluePrint/myGameMode` (`GameplayStatics.GetGameMode`))
    (:`then`
      (set `self.AsMyGameMode` _asmy_game_mode))
    (:`CastFailed`
      _))
  (bind _asmy_game_state (cast `/Game/BluePrint/myGameState` (`GameplayStatics.GetGameState`)))
  (set `self.AsMyGameState` _asmy_game_state))

(event `self.Box.OnComponentBeginOverlap`
  (params (OverlappedComponent :type "PrimitiveComponent Object Reference") (OtherActor :type "Actor Object Reference") (OtherComp :type "PrimitiveComponent Object Reference") (OtherBodyIndex :type Integer) (bFromSweep :type Boolean) (SweepResult :type "HitResult Structure (by ref)"))
  (bind _asthief (cast `/Game/BluePrint/Character/thief` OtherActor))
  (if (== (`Controller.K2_GetPawn` (`GameplayStatics.GetPlayerController` 0)) _asthief)
    (bind _asmy_game_state (cast `/Game/BluePrint/myGameState` (`GameplayStatics.GetGameState`)))
    (if (`/Game/BluePrint/myGameState.iskeyCollected?` _asmy_game_state)
      (`/Game/BluePrint/myGameState.printInstruction` _asmy_game_state "Press U to unlock the Jail")
      (set `/Game/BluePrint/Character/thief.isInRangeOfLockWithKey` true _asthief)
      (else
        (`/Game/BluePrint/myGameState.printInstruction` _asmy_game_state "First Collect the Key")))))

(fn `UserConstructionScript`)