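; Key pickup actor that tracks when the local player's thief is within reach and supports removal of the key.
; Box overlap events set and clear IsInRangeOfKey on the game state, and entering shows a press-P prompt if the key is uncollected.
; The test event calls destorykey, which destroys the game mode's Key reference rather than itself, intended to run on the server.
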(event `test`
  ;[1 1 1] Destory Actor form Server
  (`self.destorykey`))

(event `destorykey`
  ;[1 1 1] Destory Actor form Server
  (bind _asmy_game_mode (cast `/Game/BluePrint/myGameMode` (`GameplayStatics.GetGameMode`)))
  (`self.K2_DestroyActor` (`/Game/BluePrint/myGameMode.key` _asmy_game_mode)))

(event `self.Box.OnComponentBeginOverlap`
  (params (OverlappedComponent :type "PrimitiveComponent Object Reference") (OtherActor :type "Actor Object Reference") (OtherComp :type "PrimitiveComponent Object Reference") (OtherBodyIndex :type Integer) (bFromSweep :type Boolean) (SweepResult :type "HitResult Structure (by ref)"))
  (bind _asthief (cast `/Game/BluePrint/Character/thief` OtherActor))
  (if (== (`Controller.K2_GetPawn` (`GameplayStatics.GetPlayerController` 0)) _asthief)
    (bind _asmy_game_state (cast `/Game/BluePrint/myGameState` (`GameplayStatics.GetGameState`)))
    (set `/Game/BluePrint/myGameState.isInRangeOfKey` true _asmy_game_state)
    (if (not (`/Game/BluePrint/myGameState.iskeyCollected?` _asmy_game_state))
      (bind _asmy_game_state_2 (cast `/Game/BluePrint/myGameState` (`GameplayStatics.GetGameState`)))
      (`/Game/BluePrint/myGameState.printInstruction` _asmy_game_state_2 "Press P to pick the Key"))))

(event `self.Box.OnComponentEndOverlap`
  (params (OverlappedComponent :type "PrimitiveComponent Object Reference") (OtherActor :type "Actor Object Reference") (OtherComp :type "PrimitiveComponent Object Reference") (OtherBodyIndex :type Integer))
  (bind _asthief (cast `/Game/BluePrint/Character/thief` OtherActor))
  (if (== (`Controller.K2_GetPawn` (`GameplayStatics.GetPlayerController` 0)) _asthief)
    (bind _asmy_game_state (cast `/Game/BluePrint/myGameState` (`GameplayStatics.GetGameState`)))
    (set `/Game/BluePrint/myGameState.isInRangeOfKey` false _asmy_game_state)))

(fn `UserConstructionScript`)