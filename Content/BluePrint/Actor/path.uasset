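; Path actor that marks a zone where the player's thief can place a track.
; A Box overlap checks that the entering thief is the first player's pawn and that the game state reports no placed path.
; It then sets an in-range flag on the game state and shows a prompt to press P to place the track.
; Leaving the box clears the flag.
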(event `self.ReceiveBeginPlay`
  ;[1 1 1] Game Mode
  (bind _asmy_game_mode (cast `/Game/BluePrint/myGameMode` (`GameplayStatics.GetGameMode`)))
  (set `self.AsMyGameMode` _asmy_game_mode))

(event `self.Box.OnComponentBeginOverlap`
  (params (OverlappedComponent :type "PrimitiveComponent Object Reference") (OtherActor :type "Actor Object Reference") (OtherComp :type "PrimitiveComponent Object Reference") (OtherBodyIndex :type Integer) (bFromSweep :type Boolean) (SweepResult :type "HitResult Structure (by ref)"))
  (bind _asthief (cast `/Game/BluePrint/Character/thief` OtherActor))
  (bind _asmy_game_state (cast `/Game/BluePrint/myGameState` (`GameplayStatics.GetGameState`)))
  (if (and (== (`Controller.K2_GetPawn` (`GameplayStatics.GetPlayerController` 0)) _asthief) (not (`/Game/BluePrint/myGameState.IsPathPlaced?` _asmy_game_state)))
    (bind _asmy_game_state_2 (cast `/Game/BluePrint/myGameState` (`GameplayStatics.GetGameState`)))
    (set `/Game/BluePrint/myGameState.isInRangeOfPath` true _asmy_game_state_2)
    (`/Game/BluePrint/myGameState.printInstruction` _asmy_game_state_2 "Press P to Place the Track")))

(event `self.Box.OnComponentEndOverlap`
  (params (OverlappedComponent :type "PrimitiveComponent Object Reference") (OtherActor :type "Actor Object Reference") (OtherComp :type "PrimitiveComponent Object Reference") (OtherBodyIndex :type Integer))
  (bind _asthief (cast `/Game/BluePrint/Character/thief` OtherActor))
  (if (== _asthief (`Controller.K2_GetPawn` (`GameplayStatics.GetPlayerController` 0)))
    (bind _asmy_game_state (cast `/Game/BluePrint/myGameState` (`GameplayStatics.GetGameState`)))
    (set `/Game/BluePrint/myGameState.isInRangeOfPath` false _asmy_game_state)))

(fn `UserConstructionScript`)