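; Dollar is a coin pickup actor that spins and adds to the game's coin count when the player's thief touches it.
; Tick runs a short delay before each yaw step on the Coin component, so it rotates in increments.
; On Coin overlap, a thief controlled by player controller 0 increments Coins on myGameState, then calls its ForServerDestroy with the pickup, apparently to route destruction through the server.
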(event `self.ReceiveTick`
  (params (DeltaSeconds :type "Float (single-precision)"))
  (`KismetSystemLibrary.Delay` 0.2)
  (`SceneComponent.K2_AddWorldRotation` (`self.coin`) (struct :`Yaw` 10.0) false false))

(event `self.coin.OnComponentBeginOverlap`
  (params (OverlappedComponent :type "PrimitiveComponent Object Reference") (OtherActor :type "Actor Object Reference") (OtherComp :type "PrimitiveComponent Object Reference") (OtherBodyIndex :type Integer) (bFromSweep :type Boolean) (SweepResult :type "HitResult Structure (by ref)"))
  (bind _asthief (cast `/Game/BluePrint/Character/thief` OtherActor))
  (bind _asmy_game_state (cast `/Game/BluePrint/myGameState` (`GameplayStatics.GetGameState`)))
  (if (== _asthief (`Controller.K2_GetPawn` (`GameplayStatics.GetPlayerController` 0)))
    (`/Engine/EditorBlueprintResources/StandardMacros.IncrementInt` (`/Game/BluePrint/myGameState.coins` _asmy_game_state)
      (:`  `
        (`/Game/BluePrint/Character/thief.forServerDestroy` _asthief self)))))

(fn `UserConstructionScript`)