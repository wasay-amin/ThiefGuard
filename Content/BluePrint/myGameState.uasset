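; Game state that creates the game HUD at BeginPlay and holds a short-lived instruction message.
; PrintInstruction stores the text and fires the Print dispatcher, whose bound event clears it after a delay.
; An unconnected Delay-based counter loop, which would show the GameEnd widget and set GameOver on myGameMode at a time limit, never runs.
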(event `self.ReceiveBeginPlay`
  (`|ExecutionSequence`
    (:`then_1`
      (bind _returnvalue (`|CreateWidget` "/Game/UI/gameUI.gameUI_C"))
      (`UserWidget.AddToViewport` _returnvalue 0))
    (:`then_2`
      (add `self.print` (delegate `CustomEvent_0`)))))

(event `CustomEvent_0`
  (`KismetSystemLibrary.Delay` 3.0)
  (set `self.instructions` ""))

(fn `printInstruction`
  (params (print :type String))
  (returns (Instructions :type String))
  (bind _output_get (set `self.instructions` print))
  (`self.print`)
  (return _output_get))

(fn `UserConstructionScript`)